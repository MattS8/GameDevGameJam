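; BP_PatrolPath is a data-holder Blueprint that defines a patrol route for NPC AI in the HideAndSeek game.
; It stores local-space PathPoints, and Get Patrol Point converts an indexed point to world space through the actor's transform.
; Get Last Point Index returns the array's final index, clamped at zero.
; The event graph and construction script contain no logic.
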(event EventBeginPlay)

(event Collision|EventActorBeginOverlap
  (params (OtherActor :type Actor%20Object%20Reference)))

(event EventTick
  (params (DeltaSeconds :type Float%20%28single-precision%29)))

(fn ConstructionScript)

(fn GetPatrolPoint
  (params (Patrol%20Point%20Index :type Integer))
  (return (Math|Transform|TransformLocation (Transformation|GetActorTransform) (Utilities|Array|Get(acopy) (Variables|PathPoints|GetPath%20Points) Patrol%20Point%20Index))))

(fn GetLastPointIndex
  (bind _path_points (Variables|PathPoints|GetPath%20Points))
  (bind _returnvalue (Utilities|Array|Length _path_points))
  (bind _returnvalue_2 (- _returnvalue 1))
  (return (Math|Integer|Clamp(Integer) _returnvalue_2 0 _returnvalue_2)))