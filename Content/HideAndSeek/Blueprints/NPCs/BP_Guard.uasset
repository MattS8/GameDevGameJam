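; BP_Guard is a guard NPC for the hide-and-seek game that can follow the player character, which it caches on BeginPlay.
; The FollowPlayer event uses AIMoveTo toward the player, or toward itself when the player is within a short distance.
; It calls itself again after a brief delay once a move succeeds, forming a polling loop; nothing in this graph starts it.
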(event Custom|Follow%20Player
  (bind _self self)
  (if (>= (Transformation|GetDistanceTo (Variables|Default|GetCharacter%20to%20Follow)) 1e+02)
    (AI|AIMoveTo self "0, 0, 0" (Variables|Default|GetCharacter%20to%20Follow) 5.0 false
      (:then
        _))
    (else
      (AI|AIMoveTo _self "0, 0, 0" _self 5.0 false
        (:then
          _))))
  (Utilities|FlowControl|Delay 0.2)
  (CallFunction|FollowPlayer))

(event EventBeginPlay
  (Variables|Default|SetCharacter%20to%20Follow (Game|GetPlayerCharacter 0)))

(fn ConstructionScript)